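; Coin pickup for an endless runner that increments the game mode's coin count, plays a sound and destroys itself when the third-person character overlaps its mesh.
; If the character's magnet is active, overlapping the sphere counts the coin immediately, sets Used to block a second count from mesh overlap, and schedules delayed destruction.
; A timeline then pulls the coin toward the player using VInterpTo plus a Slide offset.
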(event OnComponentBeginOverlap(Sphere)
  (params (OverlappedComponent :type Primitive%20Component%20Object%20Reference) (OtherActor :type Actor%20Object%20Reference) (OtherComp :type Primitive%20Component%20Object%20Reference) (OtherBodyIndex :type Integer) (bFromSweep :type Boolean) (SweepResult :type Hit%20Result%20Structure%20%28by%20ref%29))
  ;[0 1 0.3438] Magnet - 사용시
  (bind _asthird_person_character (Utilities|Casting|CastToThirdPersonCharacter OtherActor))
  (if (Variables|/Game/MyEndlessRunner/Pawn/ThirdPersonCharacter.ThirdPersonCharacter_C|GetMagnetActive _asthird_person_character)
    (Utilities|FlowControl|Sequence
      (:then_0
        ;[1 0 0.1406] Magnet 사용 시, 이미 먹은 코인 중복 계산 방지. (Used 변수 참고)
        (bind _asthird_person_game_mode (Utilities|Casting|CastToThirdPersonGameMode (Game|GetGameMode)))
        (Math|Integer|IncrementInt (Variables|/Game/MyEndlessRunner/GameMode/ThirdPersonGameMode.ThirdPersonGameMode_C|GetCoins _asthird_person_game_mode)
          (:%20%20
            (Variables|Default|SetUsed true)
            (Audio|SpawnSound2D "/Game/MyEndlessRunner/SFX/Pickup_SFX.Pickup_SFX" 1.0 1.0 0.0 0)
            (Utilities|FlowControl|Delay 1.0)
            (Actor|DestroyActor))))
      (:then_1
        ;[0 1 0.6953] 코인이 날아가야 할 케릭터 위치 계산
        (bind _slide (Timeline|타임라인_0 PlayFromStart)
          (:Update
            (Transformation|SetActorLocation (+ _slide (Math|Interpolation|VInterpTo (.location (Transformation|GetActorTransform)) (Transformation|GetActorLocation (Game|GetPlayerCharacter 0)) (Utilities|Time|GetWorldDeltaSeconds) 15.0)) false false)))))))

(event OnComponentBeginOverlap(StaticMesh)
  (params (OverlappedComponent :type Primitive%20Component%20Object%20Reference) (OtherActor :type Actor%20Object%20Reference) (OtherComp :type Primitive%20Component%20Object%20Reference) (OtherBodyIndex :type Integer) (bFromSweep :type Boolean) (SweepResult :type Hit%20Result%20Structure%20%28by%20ref%29))
  (Utilities|Casting|CastToThirdPersonCharacter OtherActor)
  (CallFunction|PickupCoins))

(fn ConstructionScript)

(fn PickupCoins
  (bind _asthird_person_game_mode (Utilities|Casting|CastToThirdPersonGameMode (Game|GetGameMode)))
  (if (not (Variables|Default|GetUsed))
    (Variables|/Game/MyEndlessRunner/GameMode/ThirdPersonGameMode.ThirdPersonGameMode_C|SetCoins _asthird_person_game_mode (+ (Variables|/Game/MyEndlessRunner/GameMode/ThirdPersonGameMode.ThirdPersonGameMode_C|GetCoins _asthird_person_game_mode) 1))
    (Audio|SpawnSound2D "/Game/MyEndlessRunner/SFX/Pickup_SFX.Pickup_SFX" 1.0 1.0 0.0 0)
    (Actor|DestroyActor)))